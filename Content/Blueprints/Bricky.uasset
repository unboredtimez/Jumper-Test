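; Bricky is a Paper2D character Blueprint that jumps on the Jump input and switches between idle and jump flipbooks.
; The Up axis event drives UpdateAnimation, which shows the Jump flipbook whenever velocity is non-zero and Idle otherwise, without checking for falling.
; A separate AnimationStateMachine function selects a flipbook by state, but only sets and returns one when falling, and nothing shown calls it.
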(event Custom|UpdateAnimation
  ;[1 1 1] Jump Animation
  (Sprite|SetFlipbook (select (> (Math|Vector|VectorLength (Transformation|GetVelocity)) 0.0) "/Game/Sprites/Animations/Jump.Jump" "/Game/Sprites/Animations/Idle.Idle")))

(event EventBeginPlay)

(event EventActorBeginOverlap
  (params (OtherActor :type Actor%20Object%20Reference)))

(event EventTick
  (params (DeltaSeconds :type Float%20%28single-precision%29)))

(event Input|ActionEvents|InputActionJump
  ;[1 1 1] Jump Action
  (:Pressed
    (Character|Jump)))

(event Input|AxisEvents|InputAxisUp
  (params (AxisValue :type Float%20%28single-precision%29))
  ;[1 1 1] Movement Trigger
  (CallFunction|UpdateAnimation))

(fn ConstructionScript)

(fn AnimationStateMachine
  (params (IsFalling :type Boolean :default false))
  (LocalVariables|SetIsFallingLocal IsFalling)
  (if (LocalVariables|GetIsFallingLocal)
    (LocalVariables|SetAnimationState "NewEnumerator1")
    (return (Utilities|Select :Index (LocalVariables|GetAnimationState) :NewEnumerator0 (Variables|Animation|GetIdleFlipbook) :NewEnumerator1 (Variables|Animation|GetJumpFlipbook)))))